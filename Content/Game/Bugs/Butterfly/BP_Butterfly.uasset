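; Catchable butterfly that wanders between fly-location markers with bobbing flight, sparkles and sound.
; Timers pick new targets and periodic landings, while a state-driven Tick moves it and timelines rotate it or align it to a sphere-traced surface before flight resumes.
; Touching the net or VR pawn triggers a temporary speed boost.
; Caught decrements the spawner's count, spawns a dead butterfly above BP_Coldrin and destroys the actor.
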(event OnComponentBeginOverlap(CollisionComponent)
  (params (OverlappedComponent :type Primitive%20Component%20Object%20Reference) (OtherActor :type Actor%20Object%20Reference) (OtherComp :type Primitive%20Component%20Object%20Reference) (OtherBodyIndex :type Integer) (bFromSweep :type Boolean) (SweepResult :type Hit%20Result%20Structure%20%28by%20ref%29))
  (if (or (== (Utilities|GetClass OtherActor) "/Game/Game/Props/ButterflyNet.ButterflyNet_C") (== (Utilities|GetClass OtherActor) "/Game/VRExpansion/Vive/Vive_PawnCharacter.Vive_PawnCharacter_C"))
    (Variables|Default|SetSpeed 0.3)
    (CallFunction|RestartFlying)
    (Utilities|Time|SetTimerbyFunctionName 0 "TempSpeed" 1e+01)))

(event Custom|RotateTowardsLocation
  (switch Utilities|FlowControl|Switch|SwitchonButterflyStates (Variables|Default|GetButterflyState)
    (:NewEnumerator0
      _)
    (:NewEnumerator1
      _))
  (Variables|Default|SetPreRotateActorRotation (Transformation|GetActorRotation))
  (Variables|Default|SetPreRorateActorLocation (Transformation|GetActorLocation))
  (bind _alpha (Timeline|Rotate PlayFromStart)
    (:Update
      (switch Utilities|FlowControl|Switch|SwitchonButterflyStates (Variables|Default|GetButterflyState)
        (:NewEnumerator0
          _)
        (:NewEnumerator1
          _))
      (Transformation|SetActorRotation (Math|Rotator|Lerp(Rotator) (Variables|Default|GetPreRotateActorRotation) (Math|Rotator|FindLookatRotation (Variables|Default|GetPreRorateActorLocation) (Variables|Default|GetTargetLocation)) _alpha)))
    (:Finished
      (CallFunction|RotateTowardsLocation))))

(event Custom|AlignToLandingSpot
  (bind _skeletalmesh (Variables|Default|GetSkeletalMesh))
  (bind _returnvalue (Transformation|GetWorldLocation _skeletalmesh))
  (if (Variables|/Game/Game/Bugs/Butterfly/BP_ButterflyLandLocations.BP_ButterflyLandLocations_C|GetHaveButterflyAt (Utilities|Array|Get(acopy) (Variables|Default|GetLandLocationsActor) (Variables|Default|Getcurrentlylandingspotindex)))
    (bind _outhit (Class|KismetSystemLibrary|SphereTraceSinglebyProfile _returnvalue _returnvalue 5e+01 "None" false (Utilities|Array|MakeArray (Variables|Default|GetButterflynet)) "None" true))
    (Variables|Default|SetLookAtPosition (.ImpactPoint (Collision|BreakHitResult _outhit)))
    (CallFunction|MoveTowardsLandingZone)
    (else
      (CallFunction|SeekLandingSpot))))

(event Custom|MoveTowardsLandingZone
  (switch Utilities|FlowControl|Switch|SwitchonButterflyStates (Variables|Default|GetButterflyState)
    (:NewEnumerator2
      (Variables|Default|SetPreRorateActorLocation (Transformation|GetActorLocation))
      (Variables|Default|SetPreRotateActorRotation (Transformation|GetActorRotation))
      (Variables|Default|SetPreRotateDownVector (Math|Vector|NegateVector (Transformation|GetActorUpVector)))
      (Variables|Default|SetPreRorateSkeleLocation (Variables|/Script/Engine.SceneComponent|GetRelativeLocation (Variables|Default|GetSkeletalMesh)))
      (Variables|Default|SetPreTransformLand (Transformation|GetActorTransform))
      (bind _alpha (Timeline|Landing PlayFromStart)
        (:Update
          (Transformation|SetActorRotation (Math|Rotator|Lerp(Rotator) (Variables|Default|GetPreRotateActorRotation) (.rotation (Class|KismetAnimationLibrary|Lookat (Variables|Default|GetPreTransformLand) (Variables|Default|GetLookAtPosition) (Variables|Default|GetPreRotateDownVector) false "0, 0, 0" 0.0)) _alpha))
          (Transformation|SetActorLocation (Math|Vector|Lerp(Vector) (Variables|Default|GetPreRorateActorLocation) (Variables|Default|GetLookAtPosition) _alpha) false false))
        (:Finished
          (Utilities|Time|SetTimerbyEvent (delegate Custom|RestartFlying) 1e+01)
          (bind _returnvalue (Utilities|Time|SetTimerbyFunctionName 0 "SeekLandingSpot" 3e+01 false (Math|Random|RandomFloatinRange 0.0 2e+01) 1e+01))
          (Variables|Default|SetSeekLandingSpotHandle _returnvalue))))))

(event Custom|RestartFlying
  (Variables|Default|SetButterflyState "NewEnumerator0")
  (Transformation|SetActorRotation "0, 0, 0")
  (CallFunction|PickNewFlyLocation)
  (bind _returnvalue (Utilities|Time|SetTimerbyFunctionName 0 "PickNewFlyLocation" 1e+01 true 0.0 3.0))
  (Variables|Default|SetPickNewFlyLocationHandle _returnvalue))

(event EventBeginPlay
  (bind _returnvalue (Utilities|Time|SetTimerbyFunctionName 0 "SwitchMovementUpDown" 1.0 true))
  (Variables|Default|SetSwitchMovementUpDownHandle _returnvalue)
  (CallFunction|GetFlyLocations)
  (CallFunction|GetLandLocations)
  (CallFunction|PickNewFlyLocation)
  (bind _returnvalue_2 (Utilities|Time|SetTimerbyFunctionName 0 "PickNewFlyLocation" 1e+01 true 0.0 3.0))
  (Variables|Default|SetPickNewFlyLocationHandle _returnvalue_2)
  (bind _returnvalue_3 (Utilities|Time|SetTimerbyFunctionName 0 "SeekLandingSpot" 3e+01 false (Math|Random|RandomFloatinRange 0.0 2e+01)))
  (Variables|Default|SetSeekLandingSpotHandle _returnvalue_3)
  (bind _returnvalue_4 (Audio|SpawnSoundAttached "/Game/Game/Sounds/Majic_Aura.Majic_Aura" (Variables|Default|GetSkeletalMesh) "None" "0, 0, 0" "0, 0, 0" "KeepRelativeOffset" true 1.0 1.0 0.0 0 0))
  (Audio|Components|Audio|Play _returnvalue_4 0.0)
  (Niagara|SpawnSystemAttached 0 (Variables|Default|GetSparkles) "None" "0, 0, 0" "0, 0, 0" "KeepRelativeOffset" true)
  (bind _returnvalue_5 (Actor|GetActorOfClass "/Game/Game/Props/BP_Coldrin.BP_Coldrin_C"))
  (Variables|Default|SetSpawnDeadbutterflyLocation (Math|Transform|MakeTransform (+ (.location (Transformation|GetActorTransform _returnvalue_5)) "0, 0,150.000000") (.rotation (Transformation|GetActorTransform _returnvalue_5)) "1,1,1"))
  (bind _returnvalue_6 (Actor|GetActorOfClass "/Game/Game/Props/ButterflyNet.ButterflyNet_C"))
  (Variables|Default|SetButterflynet _returnvalue_6)
  (Components|Activation|Activate (Variables|Default|GetDeathCloud) false)
  (Audio|PlaySoundatLocation "/Game/Game/Sounds/ButterflyPoof_Spawn.ButterflyPoof_Spawn" (Transformation|GetActorLocation) "0, 0, 0" 1.0 1.0 0.0 0 0 0))

(event EventTick
  (params (DeltaSeconds :type Float%20%28single-precision%29))
  (bind _returnvalue (Transformation|GetActorLocation))
  (bind _returnvalue_2 (Game|GetPlayerCameraManager 0))
  (bind _returnvalue_3 (Transformation|GetActorLocation _returnvalue_2))
  (bind _returnvalue_4 (Math|Rotator|FindLookatRotation _returnvalue _returnvalue_3))
  (switch Utilities|FlowControl|Switch|SwitchonButterflyStates (Variables|Default|GetButterflyState)
    (:NewEnumerator0
      (Pawn|Input|AddMovementInput (Transformation|GetActorForwardVector) (Variables|Default|GetSpeed) false :!label _label)
      (CallFunction|BobUpandDown))
    (:NewEnumerator1
      (bind _output_get (Variables|Default|SetDistanceToLandingPoint (Math|Vector|Distance(Vector) (Variables|Default|GetTargetLocation) (Transformation|GetActorLocation))))
      (if (> _output_get 5e+01)
        (goto _label)
        (else
          (Variables|Default|SetButterflyState "NewEnumerator2")
          (CallFunction|AligntoLandingSpot))))
    (:NewEnumerator3
      (CallFunction|BobUpandDown)
      (Physics|SetSimulatePhysics (Variables|Default|GetCollisionComponent) false)
      (Transformation|SetActorRotation (Math|Rotator|MakeRotator (.roll _returnvalue_4) (.pitch _returnvalue_4) (.yaw _returnvalue_4))))))

(fn ConstructionScript)

(fn SwitchMovementUpDown
  (Variables|Default|SetbMoveUp (not (Variables|Default|GetbMoveUp))))

(fn BobUpandDown
  (if (Variables|Default|GetbMoveUp)
    (Transformation|AddActorWorldOffset (Math|Vector|MakeVector 0.0 0.0 (Math|Random|RandomFloatinRange 0.05 0.17)) true)
    (else
      (Transformation|AddActorWorldOffset (Math|Vector|MakeVector 0.0 0.0 (Math|Random|RandomFloatinRange -0.05 -0.17)) true))))

(fn GetFlyLocations
  (Utilities|Array|Clear (Variables|Default|GetFlyLocations))
  (bind _outactors (Actor|GetAllActorsOfClass "/Game/Game/Bugs/Butterfly/BP_ButterflyFlyLocation.BP_ButterflyFlyLocation_C"))
  (for _array_element _outactors
    (Utilities|Array|Add (Variables|Default|GetFlyLocations) (Transformation|GetActorLocation _array_element))))

(fn GetLandLocations
  (Utilities|Array|Clear (Variables|Default|GetLandLocations))
  (bind _outactors (Actor|GetAllActorsOfClass "/Game/Game/Bugs/Butterfly/BP_ButterflyLandLocations.BP_ButterflyLandLocations_C"))
  (for _array_element _outactors
    (Utilities|Array|Add (Variables|Default|GetLandLocations) (Transformation|GetActorLocation _array_element))
    (Utilities|Array|Add (Variables|Default|GetLandLocationsActor) _array_element)))

(fn PickNewFlyLocation
  (LocalVariables|SetTempRandomIndex (.OutIndex (Utilities|Array|Random (Variables|Default|GetFlyLocations))))
  (if (and (== (Variables|Default|GetRandomIndex) (LocalVariables|GetTempRandomIndex)) (!= (Utilities|Array|Length (Variables|Default|GetFlyLocations)) 1))
    (CallFunction|PickNewFlyLocation)
    (return)
    (else
      (bind _output_get (Variables|Default|SetRandomIndex (LocalVariables|GetTempRandomIndex)))
      (Variables|Default|SetTargetLocation (Utilities|Array|Get(acopy) (Variables|Default|GetFlyLocations) _output_get))
      (CallFunction|RotateTowardsLocation))))

(fn SeekLandingSpot
  (bind _landlocations (Variables|Default|GetLandLocations))
  (bind (_outitem _outindex) (Utilities|Array|Random _landlocations))
  (Variables|Default|SetTargetLocation _outitem)
  (Variables|Default|Setcurrentlylandingspotindex _outindex)
  (CallFunction|RotateTowardsLocation)
  (Utilities|Time|ClearandInvalidateTimerbyHandle (Variables|Default|GetPickNewFlyLocationHandle))
  (Variables|Default|SetButterflyState "NewEnumerator1"))

(fn Caught
  (Audio|PlaySoundatLocation "/Game/Game/Sounds/ButterflyPoof.ButterflyPoof" (Transformation|GetActorLocation) "0, 0, 0" 1.0 1.0 0.0 0 0 0)
  (bind _returnvalue (Actor|GetActorOfClass "/Game/Game/Bugs/Butterfly/BP_ButterflySpawner.BP_ButterflySpawner_C"))
  (Utilities|IsValid _returnvalue
    (:Is%20Valid
      (Variables|/Game/Game/Bugs/Butterfly/BP_ButterflySpawner.BP_ButterflySpawner_C|SetActiveButterflyCount _returnvalue (- (Variables|/Game/Game/Bugs/Butterfly/BP_ButterflySpawner.BP_ButterflySpawner_C|GetActiveButterflyCount _returnvalue) 1)))
    (:Is%20Not%20Valid
      _))
  (Game|SpawnActorfromClass "/Game/Game/Props/BP_DeadButterfly.BP_DeadButterfly_C" (Variables|Default|GetSpawnDeadbutterflyLocation) "Undefined" 0 0)
  (Audio|PlaySoundatLocation "/Game/Game/Sounds/ButterflyPoof.ButterflyPoof" (.location (Variables|Default|GetSpawnDeadbutterflyLocation)) "0, 0, 0" 1.0 1.0 0.0 0 0 0)
  (Actor|DestroyActor))

(fn TempSpeed
  (Variables|Default|SetSpeed 0.1))