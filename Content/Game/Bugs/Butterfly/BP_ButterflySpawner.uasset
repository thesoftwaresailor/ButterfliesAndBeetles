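; Garden spawner actor that populates the area around it with AI-controlled BP_Butterfly pawns and also triggers game over.
; An initial batch spawns at BeginPlay, then a looping timer adds one with a poof sound whenever FlowerPower exceeds the butterfly count.
; A faster timer re-sums FlowerPower from cached BP_Flower actors.
; A non-positive running total during that sum fades out, saves the score to VRGameInstance and opens MainMenuMap.
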(event Custom|SpawnInitialButterflies
  (for _index (range 0 5)
    (bind _output_get (Variables|Default|Setspawnlocation (Math|Random|RandomPointinBoundingBox (Transformation|GetActorLocation) "400.000000,400.000000,30.000000")))
    (bind _returnvalue (Game|SpawnActorfromClass "/Game/Game/Bugs/Butterfly/BP_Butterfly.BP_Butterfly_C" (Math|Transform|MakeTransform _output_get (Transformation|GetActorRotation) "1,1,1") "Undefined" 0 "NewEnumerator0" 0))
    (Pawn|SpawnDefaultController _returnvalue)
    (Math|Integer|IncrementInt (Variables|Default|GetActiveButterflyCount))))

(event EventBeginPlay
  (CallFunction|GetFlowerPower)
  (CallFunction|SpawnInitialButterflies)
  (bind _returnvalue (Utilities|Time|SetTimerbyFunctionName 0 "SpawnButterfly" 5.0 true 0.0 2.0))
  (Variables|Default|SetSpawnButterfliesHandle _returnvalue)
  (Utilities|Time|SetTimerbyFunctionName 0 "GetFlowerPower" 0.5 true)
  (bind _outactors (Actor|GetAllActorsOfClass "/Game/Game/Plants/BP_Flower.BP_Flower_C"))
  (Variables|Default|SetFlowers _outactors))

(event Collision|EventActorBeginOverlap
  (params (OtherActor :type Actor%20Object%20Reference)))

(event EventTick
  (params (DeltaSeconds :type Float%20%28single-precision%29)))

(fn ConstructionScript)

(fn SpawnButterfly
  (if (> (Variables|Default|GetFlowerPower) (Variables|Default|GetActiveButterflyCount))
    ;[1 1 1] Spawn
    (bind _output_get (Variables|Default|Setspawnlocation (Math|Random|RandomPointinBoundingBox (Transformation|GetActorLocation) "400.000000,400.000000,30.000000")))
    (Audio|PlaySoundatLocation "/Game/Game/Sounds/ButterflyPoof.ButterflyPoof" _output_get "0, 0, 0" 1.0 1.0 0.0 0 0 0)
    (bind _returnvalue (Game|SpawnActorfromClass "/Game/Game/Bugs/Butterfly/BP_Butterfly.BP_Butterfly_C" (Math|Transform|MakeTransform (Variables|Default|Getspawnlocation) (Math|Random|RandomRotator false) "1,1,1") "Undefined" 0 "NewEnumerator0" 0))
    (Pawn|SpawnDefaultController _returnvalue)
    (Math|Integer|IncrementInt (Variables|Default|GetActiveButterflyCount))))

(fn GetFlowerPower
  (Variables|Default|SetFlowerPower 0)
  (for _array_element (Variables|Default|GetFlowers)
    (bind _localflowerpower (Default|GetLocalFlowerPower _array_element))
    (bind _output_get (Variables|Default|SetFlowerPower (+ _localflowerpower (Variables|Default|GetFlowerPower))))
    (if (not (> _output_get 0))
      (if (not (Variables|Default|GetDead))
        (Variables|Default|SetDead true)
        (Audio|PlaySound2D "/Game/Game/Sounds/VoiceLines/YourFired_Cue.YourFired_Cue" 1.0 1.0 0.0 0 0)
        (CameraFades|StartCameraFade :self (Game|GetPlayerCameraManager 0) :ToAlpha 1.0 :Duration 5.5 :bShouldFadeAudio true :bHoldWhenFinished true)
        (bind _returnvalue (Actor|GetActorOfClass "/Game/Game/Score/BP_ScoreController.BP_ScoreController_C"))
        (bind _asvrgame_instance (Utilities|Casting|CastToVRGameInstance (Game|GetGameInstance)))
        (Default|SetHighestScore _asvrgame_instance (Variables|/Game/Game/Score/BP_ScoreController.BP_ScoreController_C|GetScore _returnvalue))
        (Utilities|Time|SetTimerbyFunctionName 0 "GoToMainMenuMap" 6.0)))))

(fn GotoMainMenuMap
  (Game|OpenLevel(byName) "MainMenuMap"))