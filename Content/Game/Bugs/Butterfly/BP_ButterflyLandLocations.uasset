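; BP_ButterflyLandLocations is an actor that, judging by its name, marks a butterfly landing spot and tracks whether butterflies are there.
; Its Sphere overlap events add and remove BP_Butterfly actors in the ButterfliesInZone array, ignoring other classes.
; HaveButterflyAt turns true when a butterfly enters and false once the last one leaves.
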(event OnComponentBeginOverlap(Sphere)
  (params (OverlappedComponent :type Primitive%20Component%20Object%20Reference) (OtherActor :type Actor%20Object%20Reference) (OtherComp :type Primitive%20Component%20Object%20Reference) (OtherBodyIndex :type Integer) (bFromSweep :type Boolean) (SweepResult :type Hit%20Result%20Structure%20%28by%20ref%29))
  (if (== (Utilities|GetClass OtherActor) "/Game/Game/Bugs/Butterfly/BP_Butterfly.BP_Butterfly_C")
    (Utilities|Array|Add (Variables|Default|GetButterfliesInZone) OtherActor)
    (Variables|Default|SetHaveButterflyAt true)))

(event OnComponentEndOverlap(Sphere)
  (params (OverlappedComponent :type Primitive%20Component%20Object%20Reference) (OtherActor :type Actor%20Object%20Reference) (OtherComp :type Primitive%20Component%20Object%20Reference) (OtherBodyIndex :type Integer))
  (if (== (Utilities|GetClass OtherActor) "/Game/Game/Bugs/Butterfly/BP_Butterfly.BP_Butterfly_C")
    (Utilities|Array|RemoveItem (Variables|Default|GetButterfliesInZone) OtherActor)
    (if (not (> (Utilities|Array|Length (Variables|Default|GetButterfliesInZone)) 0))
      (Variables|Default|SetHaveButterflyAt false))))

(event EventBeginPlay)

(event Collision|EventActorBeginOverlap
  (params (OtherActor :type Actor%20Object%20Reference)))

(event EventTick
  (params (DeltaSeconds :type Float%20%28single-precision%29)))

(fn ConstructionScript)