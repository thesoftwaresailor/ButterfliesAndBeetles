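; Butterfly actor that flies constantly forward while steering between fly location markers placed in the level.
; A looping timer picks a random fly location different from the last, and a self-restarting timeline repeatedly lerps rotation toward it.
; Each tick bobs the skeletal mesh by the MoveUp flag; another timer calls SwitchMovementUpDown, which is not defined here.
; Land locations are also cached at BeginPlay but not used here.
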(event Custom|RotateTowardsLocation
  (Variables|Default|SetPreRotateActorRotation (Transformation|GetActorRotation))
  (Variables|Default|SetPreRorateActorLocation (Transformation|GetActorLocation))
  (bind _alpha (Timeline|Timeline_0 PlayFromStart)
    (:Update
      (Transformation|SetActorRotation (Math|Rotator|Lerp(Rotator) (Variables|Default|GetPreRotateActorRotation) (Math|Rotator|FindLookatRotation (Variables|Default|GetPreRorateActorLocation) (Variables|Default|GetTargetLocation)) _alpha)))
    (:Finished
      (CallFunction|RotateTowardsLocation))))

(event EventBeginPlay
  (bind _returnvalue (Utilities|Time|SetTimerbyFunctionName 0 "SwitchMovementUpDown" 1.0 true))
  (Variables|Default|SetSwitchMovementUpDownHandle _returnvalue)
  (CallFunction|GetFlyLocations)
  (CallFunction|GetLandLocations)
  (CallFunction|PickNewFlyLocation)
  (bind _returnvalue_2 (Utilities|Time|SetTimerbyFunctionName 0 "PickNewFlyLocation" 1e+01 true))
  (Variables|Default|SetPickNewFlyLocationHandle _returnvalue_2))

(event Collision|EventActorBeginOverlap
  (params (OtherActor :type Actor%20Object%20Reference)))

(event EventTick
  (params (DeltaSeconds :type Float%20%28single-precision%29))
  (Transformation|AddActorWorldOffset (* (Transformation|GetActorForwardVector) 1.5))
  (CallFunction|BobUpandDown))

(fn ConstructionScript)

(fn BobUpandDown
  (if (Variables|Default|GetbMoveUp)
    (Transformation|AddLocalOffset (Variables|Default|GetSkeletalMesh) "0, 0,0.750000" false false)
    (else
      (Transformation|AddLocalOffset (Variables|Default|GetSkeletalMesh) "0, 0,-0.750000" false false))))

(fn GetFlyLocations
  (Utilities|Array|Clear (Variables|Default|GetFlyLocations))
  (bind _outactors (Actor|GetAllActorsOfClass "/Game/Game/Bugs/Butterfly/BP_ButterflyFlyLocation.BP_ButterflyFlyLocation_C"))
  (for _array_element _outactors
    (Utilities|Array|Add (Variables|Default|GetFlyLocations) (Transformation|GetActorLocation _array_element))))

(fn GetLandLocations
  (Utilities|Array|Clear (Variables|Default|GetLandLocations))
  (bind _outactors (Actor|GetAllActorsOfClass "/Game/Game/Bugs/Butterfly/BP_ButterflyLandLocations.BP_ButterflyLandLocations_C"))
  (for _array_element _outactors
    (Utilities|Array|Add (Variables|Default|GetLandLocations) (Transformation|GetActorLocation _array_element))))

(fn PickNewFlyLocation
  (LocalVariables|SetTempRandomIndex (.OutIndex (Utilities|Array|Random (Variables|Default|GetFlyLocations))))
  (if (== (Variables|Default|GetRandomIndex) (LocalVariables|GetTempRandomIndex))
    (CallFunction|PickNewFlyLocation)
    (return)
    (else
      (bind _output_get (Variables|Default|SetRandomIndex (LocalVariables|GetTempRandomIndex)))
      (Variables|Default|SetTargetLocation (Utilities|Array|Get(acopy) (Variables|Default|GetFlyLocations) _output_get))
      (CallFunction|RotateTowardsLocation))))