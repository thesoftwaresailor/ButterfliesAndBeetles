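; BP_ButterflyFlyLocation is a fly-location actor that makes butterflies choose a new destination when they reach it.
; On overlap with an actor whose class is exactly BP_ActorButterfly, it clears that butterfly's PickNewFlyLocationHandle timer and calls PickNewFlyLocation immediately.
; The destination choice itself lives in the butterfly.
; An unconnected copy of the same logic for BP_Butterfly remains in the graph and never runs.
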(event EventBeginPlay)

(event Collision|EventActorBeginOverlap
  (params (OtherActor :type Actor%20Object%20Reference))
  (if (== (Utilities|GetClass OtherActor) "/Game/Game/Bugs/Butterfly/BP_ActorButterfly.BP_ActorButterfly_C")
    (bind _asbp_actor_butterfly (Utilities|Casting|CastToBP_ActorButterfly OtherActor))
    (Utilities|Time|ClearandInvalidateTimerbyHandle (Variables|/Game/Game/Bugs/Butterfly/BP_ActorButterfly.BP_ActorButterfly_C|GetPickNewFlyLocationHandle _asbp_actor_butterfly))
    (Default|PickNewFlyLocation _asbp_actor_butterfly)))

(event EventTick
  (params (DeltaSeconds :type Float%20%28single-precision%29)))

(fn ConstructionScript)