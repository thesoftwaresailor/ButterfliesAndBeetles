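; Beetle enemy that emerges from the ground, crawls to the tree roots it is given and bites them until it dies.
; After an emerge timeline, line traces pick the nearest axis-aligned wall, then a point above it, then the ceiling toward the roots.
; Tick steers a floating movement component along that floor, wall and ceiling path, pivoting at each turn.
; On arrival it registers with the roots, plays bite effects and stops ticking; death unregisters it.
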(event Custom|Emerge
  (bind _returnvalue (Transformation|GetActorLocation))
  (Variables|Default|SetSpawnLocation _returnvalue)
  (Variables|Default|SetSpawnGroundLocation (+ _returnvalue "0, 0,25.000000"))
  (bind (_direction _emergetrack _emergerotatetrack) (Timeline|EmergeTimeline PlayFromStart)
    (:Update
      (Transformation|SetActorLocation (Math|Vector|Lerp(Vector) (Variables|Default|GetSpawnLocation) (Variables|Default|GetSpawnGroundLocation) _emergetrack) false false)
      (Transformation|SetActorRotation (Math|Rotator|Lerp(Rotator) "0.000000,0.000000,-90.000000" "0, 0, 0" _emergerotatetrack)))
    (:Finished
      (CallFunction|GetNextTarget)
      (Variables|Default|SetbIsOrienting true)
      (Variables|Default|SetbHasSpawned true))))

(event Custom|OrientBeetle
  (CallFunction|RotateBeetle))

(event Custom|PlayBiteSound
  (if (Variables|Default|GetbReachedRoots)
    (Audio|Components|Audio|Stop (Variables|Default|GetAttachedSound))
    (Audio|Components|Audio|SetSound (Variables|Default|GetAttachedSound) (Variables|Default|GetBiteSound))
    (Audio|Components|Audio|Play (Variables|Default|GetAttachedSound) 0.0)))

(event Custom|PlayCrawlSound
  (bind _returnvalue (Audio|SpawnSoundAttached (Variables|Default|GetCrawlSound) (Variables|Default|GetBody) "None" "0, 0, 0" "0, 0, 0" "KeepRelativeOffset" false 1.0 1.0 0.0 0 0))
  (Variables|Default|SetAttachedSound _returnvalue))

(event Custom|SetTargetRoots
  (params (NewTargetRoots :type BP%20Root%20Object%20Reference))
  (Variables|Default|SetTargetRoots NewTargetRoots))

(event Custom|Die
  (if (Variables|Default|GetbReachedRoots)
    (Default|RemoveBitinBeetle (Variables|Default|GetTargetRoots)))
  (Audio|Components|Audio|Stop (Variables|Default|GetAttachedSound))
  (Audio|PlaySoundatLocation "/Game/Game/Sounds/Krotos_-_Hand_to_Hand_Combat_-_Body_Hit__Bone_Break.Krotos_-_Hand_to_Hand_Combat_-_Body_Hit__Bone_Break" (Transformation|GetActorLocation) "0, 0, 0" 1.0 1.0 0.0 0 0 0)
  (Actor|DestroyActor))

(event EventBeginPlay
  (CallFunction|Emerge)
  (CallFunction|PlayCrawlSound))

(event EventTick
  (params (DeltaSeconds :type Float%20%28single-precision%29))
  (if (and (Variables|Default|GetbHasSpawned) (not (Variables|Default|GetbReachedRoots)))
    (if (Variables|Default|GetbIsOrienting)
      (CallFunction|OrientBeetle))
    (CallFunction|UpdateMovement)
    (CallFunction|CheckifReachedTarget)))

(fn ConstructionScript)

(fn UpdateMovement
  (bind _returnvalue (Transformation|GetActorLocation))
  (bind _reachoffset (Variables|Default|GetReachOffset))
  (bind _targetlocation (Variables|Default|GetTargetLocation))
  (bind _returnvalue_2 (- _targetlocation _returnvalue))
  (bind _returnvalue_3 (Math|Vector|VectorLength _returnvalue_2))
  (if (< _returnvalue_3 _reachoffset)
    (Class|NavMovementComponent|StopActiveMovement (Variables|Default|GetFloatingMovementComp) :!label _label)
    (elif (and (< _returnvalue_3 (* _reachoffset 18.0)) (Variables|Default|GetbIsClimbingCeiling))
      (goto _label)
      (else
        (Class|PawnMovementComponent|AddInputVector (Variables|Default|GetFloatingMovementComp) (Math|Vector|ClampVectorSize _returnvalue_2 0.0 2.0) false)))))

(fn CheckifReachedTarget
  (if (Math|Vector|Equal(Vector) (Transformation|GetActorLocation) (Variables|Default|GetTargetLocation) 2.0)
    (if (Variables|Default|GetbIsOnFloor)
      (CallFunction|PivotBeetle)
      (Variables|Default|SetbIsOnFloor false)
      (Variables|Default|SetbIsClimbingWall true)
      (CallFunction|GetNextTarget)
      (elif (Variables|Default|GetbIsClimbingWall)
        (CallFunction|PivotBeetle)
        (Variables|Default|SetbIsClimbingWall false)
        (Variables|Default|SetbIsClimbingCeiling true)
        (CallFunction|GetNextTarget)
        (else
          (Variables|Default|SetbReachedRoots true :!label _label)
          (Components|Animation|PlayAnimation (Variables|Default|GetBeetleSkeleton) "/Game/Game/Bugs/BettalBite_Anim.BettalBite_Anim" true)
          (Audio|Components|Audio|Stop (Variables|Default|GetAttachedSound))
          (CallFunction|PlayBiteSound)
          (Default|AddBitinBeetle (Variables|Default|GetTargetRoots))
          (Components|Activation|Activate (Variables|Default|GetEatingCloud) false)
          (Actor|Tick|SetActorTickEnabled false))))
    (elif (and (Math|Vector|Equal(Vector) (Transformation|GetActorLocation) (Variables|Default|GetTargetLocation) 12.0) (Variables|Default|GetbIsClimbingCeiling))
      (goto _label))))

(fn GetNextTarget
  (bind _returnvalue (Transformation|GetActorLocation))
  (if (Variables|Default|GetbIsOnFloor)
    (CallFunction|FloorTargetTrace)
    (switch Utilities|FlowControl|Switch|SwitchonEBeetleDirection (Variables|Default|GetDirection)
      (:NewEnumerator0
        (Variables|Default|SetTargetRotation "0,90.000000, 0"))
      (:NewEnumerator1
        (Variables|Default|SetTargetRotation "0, 0, 0"))
      (:NewEnumerator2
        (Variables|Default|SetTargetRotation "0,-90.000000, 0"))
      (:NewEnumerator3
        (Variables|Default|SetTargetRotation "0,180.000000, 0")))
    (elif (Variables|Default|GetbIsClimbingWall)
      (bind _outhit (Collision|LineTraceByChannel _returnvalue (+ _returnvalue "0,0.000000,500.000000") "TraceTypeQuery5" false 0 "ForOneFrame"))
      (Variables|Default|SetTargetLocation (- (.Location (Collision|BreakHitResult _outhit)) "0,0.000000,25.000000"))
      (else
        (bind _outhit_2 (Collision|LineTraceByChannel (Transformation|GetActorLocation) (Transformation|GetActorLocation (Variables|Default|GetTargetRoots)) "TraceTypeQuery5" false 0 "ForOneFrame"))
        (Variables|Default|SetTargetLocation (- (.Location (Collision|BreakHitResult _outhit_2)) "0, 0,5.000000"))))))

(fn FloorTargetTrace
  (bind _returnvalue (Transformation|GetActorLocation))
  (bind _returnvalue_2 (Transformation|GetActorLocation))
  (bind _returnvalue_3 (Transformation|GetActorLocation))
  (bind _returnvalue_4 (Transformation|GetActorLocation))
  (bind (_outhit _returnvalue_5) (Collision|LineTraceByChannel _returnvalue_4 (+ _returnvalue_4 "500.000000, 0, 0" "") "TraceTypeQuery5" false 0 "ForOneFrame"))
  (if _returnvalue_5
    (LocalVariables|SetShortestDistance (.Distance (Collision|BreakHitResult _outhit)))
    (Variables|Default|SetTargetLocation (- (.Location (Collision|BreakHitResult _outhit)) "25.000000, 0, 0"))
    (Variables|Default|SetDirection "NewEnumerator0"))
  (bind (_outhit_2 _returnvalue_6) (Collision|LineTraceByChannel _returnvalue (+ _returnvalue "0.000000,500.000000,0.000000") "TraceTypeQuery5" false 0 "ForOneFrame"))
  (if _returnvalue_6
    (if (< (.Distance (Collision|BreakHitResult _outhit_2)) (LocalVariables|GetShortestDistance))
      (LocalVariables|SetShortestDistance (.Distance (Collision|BreakHitResult _outhit_2)))
      (Variables|Default|SetTargetLocation (- (.Location (Collision|BreakHitResult _outhit_2)) "0,25.000000,0.000000"))
      (Variables|Default|SetDirection "NewEnumerator1")))
  (bind (_outhit_3 _returnvalue_7) (Collision|LineTraceByChannel _returnvalue_3 (- _returnvalue_3 "500.000000, 0, 0") "TraceTypeQuery5" false 0 "ForOneFrame"))
  (if _returnvalue_7
    (if (< (.Distance (Collision|BreakHitResult _outhit_3)) (LocalVariables|GetShortestDistance))
      (LocalVariables|SetShortestDistance (.Distance (Collision|BreakHitResult _outhit_3)))
      (Variables|Default|SetTargetLocation (+ (.Location (Collision|BreakHitResult _outhit_3)) "25.000000, 0, 0"))
      (Variables|Default|SetDirection "NewEnumerator2")))
  (bind (_outhit_4 _returnvalue_8) (Collision|LineTraceByChannel _returnvalue_2 (- _returnvalue_2 "0.000000,500.000000,0.000000") "TraceTypeQuery5" false 0 "ForOneFrame"))
  (if _returnvalue_8
    (if (< (.Distance (Collision|BreakHitResult _outhit_4)) (LocalVariables|GetShortestDistance))
      (LocalVariables|SetShortestDistance (.Distance (Collision|BreakHitResult _outhit_4)))
      (Variables|Default|SetTargetLocation (+ (.Location (Collision|BreakHitResult _outhit_4)) "0.000000,25.000000,0.000000"))
      (Variables|Default|SetDirection "NewEnumerator3"))))

(fn PivotBeetle
  (LocalVariables|SetVelX (.x (Variables|/Script/Engine.MovementComponent|GetVelocity (Variables|Default|GetFloatingMovementComp))))
  (LocalVariables|SetVelY (.y (Variables|/Script/Engine.MovementComponent|GetVelocity (Variables|Default|GetFloatingMovementComp))))
  (LocalVariables|SetVelZ (.z (Variables|/Script/Engine.MovementComponent|GetVelocity (Variables|Default|GetFloatingMovementComp))))
  (if (Variables|Default|GetbIsClimbingWall)
    (Variables|/Script/Engine.MovementComponent|SetVelocity (Variables|Default|GetFloatingMovementComp) (Math|Vector|MakeVector (LocalVariables|GetVelX) (LocalVariables|GetVelY) 0.0))
    (switch Utilities|FlowControl|Switch|SwitchonEBeetleDirection (Variables|Default|GetDirection)
      (:NewEnumerator0
        (Variables|Default|SetTargetRotation (Math|Rotator|CombineRotators (Variables|Default|GetTargetRotation) "90.000000, 0,0.000000")))
      (:NewEnumerator1
        (Variables|Default|SetTargetRotation (Math|Rotator|CombineRotators (Variables|Default|GetTargetRotation) "0, 0,90.000000")))
      (:NewEnumerator2
        (Variables|Default|SetTargetRotation (Math|Rotator|CombineRotators (Variables|Default|GetTargetRotation) "270.000000, 0,0.000000")))
      (:NewEnumerator3
        (Variables|Default|SetTargetRotation (Math|Rotator|CombineRotators (Variables|Default|GetTargetRotation) "0.000000, 0,-90.000000"))))
    (else
      (switch Utilities|FlowControl|Switch|SwitchonEBeetleDirection (Variables|Default|GetDirection)
        (:NewEnumerator0
          (Variables|Default|SetTargetRotation (Math|Rotator|CombineRotators (Variables|Default|GetTargetRotation) "90.000000, 0,0.000000"))
          (Variables|/Script/Engine.MovementComponent|SetVelocity (Variables|Default|GetFloatingMovementComp) (Math|Vector|MakeVector 0.0 (LocalVariables|GetVelY) (LocalVariables|GetVelZ)) :!label _label))
        (:NewEnumerator1
          (Variables|Default|SetTargetRotation (Math|Rotator|CombineRotators (Variables|Default|GetTargetRotation) "0, 0,90.000000"))
          (Variables|/Script/Engine.MovementComponent|SetVelocity (Variables|Default|GetFloatingMovementComp) (Math|Vector|MakeVector (LocalVariables|GetVelX) 0.0 (LocalVariables|GetVelZ)) :!label _label_2))
        (:NewEnumerator2
          (Variables|Default|SetTargetRotation (Math|Rotator|CombineRotators (Variables|Default|GetTargetRotation) "270.000000, 0,0.000000"))
          (goto _label))
        (:NewEnumerator3
          (Variables|Default|SetTargetRotation (Math|Rotator|CombineRotators (Variables|Default|GetTargetRotation) "0.000000, 0,-90.000000"))
          (goto _label_2)))))
  (Variables|Default|SetbIsOrienting true))

(fn RotateBeetle
  (bind _returnvalue (Transformation|GetActorRotation))
  (bind _returnvalue_2 (Transformation|GetActorRotation))
  (bind _targetrotation (Variables|Default|GetTargetRotation))
  (bind _targetrotation_2 (Variables|Default|GetTargetRotation))
  (bind _returnvalue_3 (Math|Float|Absolute(Float) (.roll _returnvalue)))
  (bind _returnvalue_4 (Math|Float|Absolute(Float) (.pitch _returnvalue)))
  (bind _returnvalue_5 (Math|Float|Absolute(Float) (.yaw _returnvalue)))
  (bind _returnvalue_6 (Math|Float|Absolute(Float) (.roll _targetrotation_2)))
  (bind _returnvalue_7 (Math|Float|Absolute(Float) (.pitch _targetrotation_2)))
  (bind _returnvalue_8 (Math|Float|Absolute(Float) (.yaw _targetrotation_2)))
  (bind _returnvalue_9 (Math|Float|NearlyEqual(Float) _returnvalue_5 _returnvalue_8 5.0))
  (bind _returnvalue_10 (Math|Float|NearlyEqual(Float) _returnvalue_3 _returnvalue_6 5.0))
  (bind _returnvalue_11 (Math|Float|NearlyEqual(Float) _returnvalue_4 _returnvalue_7 5.0))
  (if (and (and _returnvalue_10 _returnvalue_11) _returnvalue_9)
    (Variables|Default|SetbIsOrienting false)
    (else
      (LocalVariables|SetRotX (.roll _returnvalue_2))
      (LocalVariables|SetRotY (.pitch _returnvalue_2))
      (LocalVariables|SetRotZ (.yaw _returnvalue_2))
      (LocalVariables|SetTarX (.roll _targetrotation))
      (LocalVariables|SetTarY (.pitch _targetrotation))
      (LocalVariables|SetTarZ (.yaw _targetrotation))
      (if _returnvalue_10
        _
        (elif (< (LocalVariables|GetTarX) (LocalVariables|GetRotX))
          (LocalVariables|SetXMod (+ (LocalVariables|GetXMod) (Variables|Default|GetTurnRate)))
          (else
            (LocalVariables|SetXMod (- (LocalVariables|GetXMod) (Variables|Default|GetTurnRate))))))
      (if _returnvalue_11
        _
        (elif (< (LocalVariables|GetTarY) (LocalVariables|GetRotY))
          (LocalVariables|SetYMod (+ (LocalVariables|GetYMod) (Variables|Default|GetTurnRate)))
          (else
            (LocalVariables|SetYMod (- (LocalVariables|GetYMod) (Variables|Default|GetTurnRate))))))
      (if _returnvalue_9
        _
        (elif (< (LocalVariables|GetTarZ) (LocalVariables|GetRotZ))
          (LocalVariables|SetZMod (+ (LocalVariables|GetZMod) (Variables|Default|GetTurnRate)))
          (else
            (LocalVariables|SetZMod (- (LocalVariables|GetZMod) (Variables|Default|GetTurnRate))))))
      (Transformation|SetActorRotation (Math|Rotator|CombineRotators (Math|Rotator|MakeRotator (LocalVariables|GetXMod) (LocalVariables|GetYMod) (LocalVariables|GetZMod)) (Transformation|GetActorRotation))))))