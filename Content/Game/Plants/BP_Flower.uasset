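; Magic flower actor that tracks a local flower power level and exposes it through a getter.
; BeginPlay creates a dynamic material instance on the flower mesh.
; WiltFlower lowers power toward zero and uses a timeline to blend FlowerPowerColor to match, assuming a hardcoded maximum of three.
; PerkUpFlower raises power up to that cap but only prints, leaving the material unchanged.
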(event Custom|WiltFlower
  (if (not (<= (Variables|Default|GetLocalFlowerPower) 0))
    (Math|Integer|DecrementInt (Variables|Default|GetLocalFlowerPower)
      (:%20%20
        (bind _returnvalue (Rendering|Material|GetScalarParameterValue (Variables|Default|GetMatreal%20Instance) "FlowerPowerColor" :!class /Script/Engine.MaterialInstanceDynamic))
        (Variables|Default|SetWiltSaturation _returnvalue)
        (Variables|Default|SetBoneRotation (Transformation|GetSocketRotation (Variables|Default|GetMagicFlower) "Bone_001"))
        (bind _newtrack_0 (Timeline|Timeline_0 PlayFromStart)
          (:Update
            (Rendering|Material|SetScalarParameterValue (Variables|Default|GetMatreal%20Instance) "FlowerPowerColor" (Math|Float|Lerp (Variables|Default|GetWiltSaturation) (Math|Float|Absolute(Float) (- (/ (Math|Conversions|ToFloat(Integer) (Variables|Default|GetLocalFlowerPower)) 3.0) 1.0)) _newtrack_0) :!class /Script/Engine.MaterialInstanceDynamic)))))))

(event Custom|PerkUpFlower
  (if (not (>= (Variables|Default|GetLocalFlowerPower) 3))
    (Math|Integer|IncrementInt (Variables|Default|GetLocalFlowerPower)
      (:%20%20
        (Development|PrintString "Perk Up")))))

(event EventBeginPlay
  (bind _returnvalue (Rendering|Material|CreateDynamicMaterialInstance (Variables|Default|GetMagicFlower) 0 "/Game/Game/Matreals/M_Flower.M_Flower" "None" :!class /Script/Engine.PrimitiveComponent))
  (Variables|Default|SetMatreal%20Instance _returnvalue))

(event Collision|EventActorBeginOverlap
  (params (OtherActor :type Actor%20Object%20Reference)))

(event EventTick
  (params (DeltaSeconds :type Float%20%28single-precision%29)))

(fn ConstructionScript)

(fn GetLocalFlowerPower
  (return (Variables|Default|GetLocalFlowerPower)))