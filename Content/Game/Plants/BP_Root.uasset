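; BP_Root is a plant root that wilts or revives its linked MagicFlower depending on the BitinBeetles attacking it.
; Events add or remove beetles from a count, which a looping half-second timer subtracts from a wilt threshold, wilting the flower and resetting at zero.
; With no beetles, an unwilt counter climbs until it perks the flower up, or marks the root dead if the flower has no power left.
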(event Custom|AddBitinBeetle
  (Math|Integer|IncrementInt (Variables|Default|GetBitinBeetles)))

(event Custom|RemoveBitinBeetle
  (Math|Integer|DecrementInt (Variables|Default|GetBitinBeetles)))

(event EventBeginPlay
  (bind _returnvalue (Utilities|Time|SetTimerbyFunctionName 0 "UpdateRootState" 0.5 true))
  (Variables|Default|SetRootStateTimer _returnvalue))

(event Collision|EventActorBeginOverlap
  (params (OtherActor :type Actor%20Object%20Reference)))

(fn ConstructionScript)

(fn UpdateRootState
  (Variables|Default|SetWiltThreshold (- (Variables|Default|GetWiltThreshold) (Variables|Default|GetBitinBeetles)))
  (if (<= (Variables|Default|GetWiltThreshold) 0)
    (Default|WiltFlower (Variables|Default|GetMagicFlower))
    (Variables|Default|SetWiltThreshold 100)
    (elif (and (== (Variables|Default|GetBitinBeetles) 0) (not (Variables|Default|GetbIsDead)))
      (Variables|Default|SetUnWiltThreshold (+ (Variables|Default|GetUnWiltThreshold) 2))
      (if (>= (Variables|Default|GetUnWiltThreshold) 100)
        (if (== (Variables|/Game/Game/Plants/BP_Flower.BP_Flower_C|GetLocalFlowerPower (Variables|Default|GetMagicFlower)) 0)
          (Variables|Default|SetbIsDead true)
          (else
            (Default|PerkUpFlower (Variables|Default|GetMagicFlower))
            (Variables|Default|SetUnWiltThreshold 0))))
      (else
        (Variables|Default|SetUnWiltThreshold 0)))))