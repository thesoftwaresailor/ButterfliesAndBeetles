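; BP_ScoreController tracks the player's score and turns earned points into physical coins at the money chest.
; On BeginPlay it caches the coin spawn box from the MoneyChest actor.
; IncrementScoreByButterflyCount adds five points per butterfly and spawns one BP_Coin per point at random positions and rotations inside that box.
; It then updates the Scoreboard and passes the score to VRGameInstance's SetHighestScore.
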(event Custom|IncrementScoreByButterflyCount
  (params (NumButterflies :type Integer))
  (bind _coin_spawn_bounding_box (Variables|Default|GetCoin%20Spawn%20Bounding%20Box))
  (Variables|Default|SetScore (+ (* NumButterflies 5) (Variables|Default|GetScore)))
  (for _index (range 0 (* NumButterflies 5))
    (Game|SpawnActorfromClass "/Game/Game/Props/BP_Coin.BP_Coin_C" (Math|Transform|MakeTransform (Math|Random|RandomPointinBoundingBox (Transformation|GetWorldLocation _coin_spawn_bounding_box) (Variables|/Script/Engine.BoxComponent|GetBoxExtent _coin_spawn_bounding_box)) (Math|Random|RandomRotator true) "1,1,1") "AdjustIfPossibleButAlwaysSpawn" 0 0))
  (Default|UpdateScore (Variables|Default|GetScoreboard) (Variables|Default|GetScore))
  (bind _asvrgame_instance (Utilities|Casting|CastToVRGameInstance (Game|GetGameInstance)))
  (Default|SetHighestScore _asvrgame_instance (Variables|Default|GetScore)))

(event EventBeginPlay
  (bind _returnvalue (Actor|GetActorOfClass "/Game/Game/Props/MoneyChest.MoneyChest_C"))
  (Variables|Default|SetCoin%20Spawn%20Bounding%20Box (Variables|/Game/Game/Props/MoneyChest.MoneyChest_C|GetCoinSpawnBoundingBox _returnvalue)))

(event Collision|EventActorBeginOverlap
  (params (OtherActor :type Actor%20Object%20Reference)))

(event EventTick
  (params (DeltaSeconds :type Float%20%28single-precision%29)))

(fn ConstructionScript)