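; Queue manager that spawns NPC customers and assigns them to storefront or waiting-line slots, registering with TimeAttack_GM on BeginPlay.
; Waves run on a temporary looping timer; new NPCs spawn at the last line point, taking a free store slot or else joining the line.
; A leave request frees the store slot and moves the line up, asking SteamVR_GM for the next wave when the line runs short.
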(event Custom|SpawnNPCWave
  (params (Count :type Integer))
  (bind _returnvalue (Utilities|Time|SetTimerbyEvent (EventDispatchers|CreateEvent :!event SpawnNPC) 2.0 true))
  (Utilities|FlowControl|Delay (+ (* Count 2.0) 0.2))
  (Utilities|Time|ClearandInvalidateTimerbyHandle _returnvalue))

(event EventBeginPlay
  (Variables|Default|SetMaxShopVisitors (Math|Integer|Min(Integer) (Utilities|Array|Length (Variables|Default|GetStoreTargetPoints)) (Variables|Default|GetMaxShopVisitors)))
  (bind _astime_attack_gm (Utilities|Casting|CastToTimeAttack_GM (Game|GetGameMode)))
  (Default|RegisterLineManager _astime_attack_gm self))

(event Collision|EventActorBeginOverlap
  (params (OtherActor :type Actor%20Object%20Reference)))

(fn ConstructionScript)

(fn SendNPCtoStore
  (params (NPC :type BP%20NPC%20Object%20Reference%20%28by%20ref%29))
  (bind (_array_element _array_index) (Utilities|Array|ForEachLoopwithBreak (Variables|Default|GetStoreTargetPoints) :!label _label)
    (:LoopBody
      (if (not (.InUse (Utilities|Struct|BreakFStoreFrontSlotData _array_element)))
        (Default|HandleRequesttoApproachStore NPC (.TargetPoint (Utilities|Struct|BreakFStoreFrontSlotData _array_element)))
        (EventDispatchers|BindEventtoOnRequestLeaveStore NPC (EventDispatchers|CreateEvent :!event OnNPCRequestLeaveStore))
        (bind _structout (Utilities|Struct|SetmembersinFStoreFrontSlotData _array_element true NPC))
        (Utilities|Array|SetArrayElem (Variables|Default|GetStoreTargetPoints) _array_index _structout)
        (goto _label Break)))))

(fn SendNPCtoFrontOfLine
  (params (NPC :type BP%20NPC%20Object%20Reference))
  (bind (_array_element _array_index) (Utilities|Array|ForEachLoopwithBreak (Variables|Default|GetLineTargetPoints) :!label _label)
    (:LoopBody
      (if (not (.InUse (Utilities|Struct|BreakFStoreFrontSlotData _array_element)))
        (Default|MovetoLineSlot NPC (.TargetPoint (Utilities|Struct|BreakFStoreFrontSlotData _array_element)))
        (bind _structout (Utilities|Struct|SetmembersinFStoreFrontSlotData _array_element true NPC))
        (Utilities|Array|SetArrayElem (Variables|Default|GetLineTargetPoints) _array_index _structout)
        (goto _label Break)))))

(fn MoveLineUp
  ;[1 1 1] Move line waiters to store
  (bind _return (CallFunction|GetAvailableStoreSlots))
  (bind _output_get (LocalVariables|SetStoreSlotsToFill _return))
  (for _index (range 0 (- _output_get 1))
    (if (.InUse (Utilities|Struct|BreakFStoreFrontSlotData (Utilities|Array|Get(acopy) (Variables|Default|GetLineTargetPoints) _index)))
      (CallFunction|SendNPCtoStore (.NPC (Utilities|Struct|BreakFStoreFrontSlotData (Utilities|Array|Get(acopy) (Variables|Default|GetLineTargetPoints) _index))))
      (Utilities|Struct|SetmembersinFStoreFrontSlotData (Utilities|Array|Get(acopy) (Variables|Default|GetLineTargetPoints) _index) false)))
  (for (_array_element _array_index) (Variables|Default|GetLineTargetPoints)
    (if (.InUse (Utilities|Struct|BreakFStoreFrontSlotData _array_element))
      (CallFunction|SendNPCtoFrontOfLine (.NPC (Utilities|Struct|BreakFStoreFrontSlotData _array_element)))
      (bind _structout (Utilities|Struct|SetmembersinFStoreFrontSlotData _array_element false))
      (Utilities|Array|SetArrayElem (Variables|Default|GetLineTargetPoints) _array_index _structout)))
  (bind _return_2 (CallFunction|GetLineLength))
  (if (< _return_2 3)
    (bind _assteam_vr_gm (Utilities|Casting|CastToSteamVR_GM (Game|GetGameMode)))
    (Default|StartNextWave _assteam_vr_gm)))

(fn SpawnNPC
  (bind _linetargetpoints (Variables|Default|GetLineTargetPoints))
  (bind _returnvalue (Game|SpawnActorfromClass "/Game/Game/AI/BP_NPC.BP_NPC_C" (Transformation|GetActorTransform (.TargetPoint (Utilities|Struct|BreakFStoreFrontSlotData (Utilities|Array|Get(acopy) _linetargetpoints (Utilities|Array|LastIndex _linetargetpoints))))) "Undefined" 0 (Variables|Default|GetScoreController) 0))
  (Utilities|IsValid _returnvalue
    (:Is%20Valid
      (bind _return (CallFunction|GetAvailableStoreSlots))
      (if (> _return 0)
        (CallFunction|SendNPCtoStore _returnvalue)
        (else
          (CallFunction|SendNPCtoFrontOfLine _returnvalue))))
    (:Is%20Not%20Valid
      (Development|PrintString "TOO MANY NPCs!"))))

(fn OnNPCRequestLeaveStore
  (params (NPC :type BP%20NPC%20Object%20Reference))
  (for (_array_element _array_index) (Variables|Default|GetStoreTargetPoints)
    (if (== NPC (.NPC (Utilities|Struct|BreakFStoreFrontSlotData _array_element)))
      (bind _structout (Utilities|Struct|SetmembersinFStoreFrontSlotData _array_element false))
      (Utilities|Array|SetArrayElem (Variables|Default|GetStoreTargetPoints) _array_index _structout)))
  (CallFunction|MoveLineUp))

(fn GetAvailableStoreSlots
  (for _array_element (Variables|Default|GetStoreTargetPoints)
    (if (not (.InUse (Utilities|Struct|BreakFStoreFrontSlotData _array_element)))
      (Math|Integer|IncrementInt (LocalVariables|GetAvailableSlotCount))))
  (return (Math|Integer|Min(Integer) (Variables|Default|GetMaxShopVisitors) (LocalVariables|GetAvailableSlotCount))))

(fn GetLineLength
  (for _array_element (Variables|Default|GetLineTargetPoints)
    (if (.InUse (Utilities|Struct|BreakFStoreFrontSlotData _array_element))
      (Math|Integer|IncrementInt (LocalVariables|Getcount))))
  (return (LocalVariables|Getcount)))