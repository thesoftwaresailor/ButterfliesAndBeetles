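; BP_NPC is a customer with a random mesh that moves to line slots or the storefront, where it reaches out to receive a jar.
; An overlapping BP_Jar containing dead butterflies scores by butterfly count, triggers a replacement from BP_JarSpawner, and plays poof and coin feedback.
; After a short delay it announces its departure, walks hardcoded waypoints, turns randomly left or right, then destroys itself.
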(event OnComponentBeginOverlap(JarReceiver)
  (params (OverlappedComponent :type Primitive%20Component%20Object%20Reference) (OtherActor :type Actor%20Object%20Reference) (OtherComp :type Primitive%20Component%20Object%20Reference) (OtherBodyIndex :type Integer) (bFromSweep :type Boolean) (SweepResult :type Hit%20Result%20Structure%20%28by%20ref%29))
  (bind _n_jarpoof (Variables|Default|GetN_JarPoof))
  (bind _asbp_jar (Utilities|Casting|CastToBP_Jar OtherActor))
  (if (> (Utilities|Array|Length (Variables|/Game/Game/Props/BP_Jar.BP_Jar_C|GetDeadbutterfly _asbp_jar)) 0)
    (Variables|Default|SetHeldJar _asbp_jar)
    (bind _returnvalue (Actor|GetActorOfClass "/Game/Game/Props/JarStuff/BP_JarSpawner.BP_JarSpawner_C"))
    (Default|SpawnJar _returnvalue)
    (Collision|SetCollisionEnabled (Variables|Default|GetJarReceiver) "NoCollision")
    (Default|IncrementScorebyButterflyCount (Variables|Default|GetScoreController) (Utilities|Array|Length (Variables|/Game/Game/Props/BP_Jar.BP_Jar_C|GetDeadbutterfly (Variables|Default|GetHeldJar))))
    (Components|Activation|Activate _n_jarpoof false)
    (Transformation|DetachFromComponent _n_jarpoof "KeepWorld" "KeepWorld" "KeepWorld" true)
    (Default|PreparedDeath (Variables|Default|GetHeldJar))
    (Audio|PlaySound2D "/Game/Game/Sounds/CoinHit.CoinHit" 1.0 1.0 0.0 0 0)
    (Utilities|FlowControl|Delay 1.0)
    (CallFunction|RequestLeaveStore)))

(event Custom|RequestLeaveStore
  (Default|CallOnRequestLeaveStore self)
  (bind _asanim_bp_npc (Utilities|Casting|CastToAnimBP_NPC (Components|SkeletalMesh|GetAnimInstance (Variables|Character|GetMesh))))
  (Variables|/Game/PolygonFantasyKingdom/Anims/AnimBP_NPC.AnimBP_NPC_C|SetbReaching _asanim_bp_npc false)
  (AI|AIMoveTo self "2403.000000,161.000000,100.000000" 0 15.0 false
    (:OnSuccess
      (AI|AIMoveTo self "6103.000000,161.000000,100.000000" 0 15.0 false
        (:OnSuccess
          (if (Math|Random|RandomBool) ; Go left or right
            (AI|AIMoveTo self "6103.000000,2468.000000,100.000000" 0 15.0 false
              (:OnSuccess
                _))
            (else
              (AI|AIMoveTo self "6103.000000,-2021.000000,100.000000" 0 15.0 false
                (:OnSuccess
                  _))))
          (Actor|DestroyActor))))))

(event Custom|MoveToStore
  (params (TargetPoint :type Target%20Point%20Object%20Reference))
  (AI|AIMoveTo self "0, 0, 0" TargetPoint 5.0 false
    (:OnSuccess
      (Transformation|SetActorRotation (Transformation|GetActorRotation TargetPoint))
      (CallFunction|OnWalktoStoreComplete))))

(event Custom|MoveToLineSlot
  (params (TargetPOint :type Actor%20Object%20Reference))
  (AI|AIMoveTo self "0, 0, 0" TargetPOint 5.0 false))

(event EventEndPlay
  (params (EndPlayReason :type EEndPlayReason%20Enum :default "Destroyed"))
  (bind _heldjar (Variables|Default|GetHeldJar)
    (:then
      (Default|PreparedDeath _heldjar))
    (:else)))

(event EventBeginPlay
  (CallFunction|ChooseRandomMesh))

(fn ConstructionScript)

(fn HandleRequesttoApproachStore
  (params (TargetPoint :type Target%20Point%20Object%20Reference))
  (CallFunction|MovetoStore TargetPoint))

(fn OnWalktoStoreComplete
  (Collision|SetCollisionEnabled (Variables|Default|GetJarReceiver) "QueryOnly")
  (Variables|Default|SetbAtStorefront true)
  (bind _asanim_bp_npc (Utilities|Casting|CastToAnimBP_NPC (Components|SkeletalMesh|GetAnimInstance (Variables|Character|GetMesh))))
  (Variables|/Game/PolygonFantasyKingdom/Anims/AnimBP_NPC.AnimBP_NPC_C|SetbReaching _asanim_bp_npc true))

(fn ChooseRandomMesh
  (bind _charactermeshes (Variables|Default|GetCharacterMeshes))
  (Class|SkinnedMeshComponent|SetSkeletalMesh (Variables|Character|GetMesh) (Utilities|Array|Get(acopy) _charactermeshes (Math|Random|RandomIntegerinRange 0 (Utilities|Array|LastIndex _charactermeshes))) true))