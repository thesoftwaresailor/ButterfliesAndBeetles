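; Ambient sound manager that switches a 2D background sound between above and below variants for the Vive pawn.
; BeginPlay starts the above sound.
; When the pawn begins or ends overlap with Collision, its height against a fixed Z threshold picks the variant, fading out the old sound and spawning the new.
; Boolean flags gate switches, but only begin overlap updates them; end overlap uses a slower fade.
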(event OnComponentEndOverlap(Collision)
  (params (OverlappedComponent :type Primitive%20Component%20Object%20Reference) (OtherActor :type Actor%20Object%20Reference) (OtherComp :type Primitive%20Component%20Object%20Reference) (OtherBodyIndex :type Integer))
  (if (== (Utilities|GetClass OtherActor) "/Game/VRExpansion/Vive/Vive_PawnCharacter.Vive_PawnCharacter_C")
    (if (>= (.z (Transformation|GetActorLocation OtherActor)) -1.1e+02)
      (if (Variables|Default|GetbIsPlayingBelowAmbient)
        (Audio|Components|Audio|FadeOut (Variables|Default|GetAudio) 1.0 0.0 "Linear" :!class /Script/Engine.AudioComponent)
        (bind _returnvalue (Audio|SpawnSound2D (Variables|Default|GetAboveAmbient) 1.0 1.0 0.0 0))
        (Variables|Default|SetAudio _returnvalue))
      (elif (Variables|Default|GetbIsPlayingAboveAmbient)
        (Audio|Components|Audio|FadeOut (Variables|Default|GetAudio) 1.0 0.0 "Linear" :!class /Script/Engine.AudioComponent)
        (bind _returnvalue_2 (Audio|SpawnSound2D (Variables|Default|GetBelowAmbient) 1.0 1.0 0.0 0))
        (Variables|Default|SetAudio _returnvalue_2)))))

(event OnComponentBeginOverlap(Collision)
  (params (OverlappedComponent :type Primitive%20Component%20Object%20Reference) (OtherActor :type Actor%20Object%20Reference) (OtherComp :type Primitive%20Component%20Object%20Reference) (OtherBodyIndex :type Integer) (bFromSweep :type Boolean) (SweepResult :type Hit%20Result%20Structure%20%28by%20ref%29))
  (if (== (Utilities|GetClass OtherActor) "/Game/VRExpansion/Vive/Vive_PawnCharacter.Vive_PawnCharacter_C")
    (if (>= (.z (Transformation|GetActorLocation OtherActor)) -1.1e+02)
      (if (Variables|Default|GetbIsPlayingBelowAmbient)
        (Audio|Components|Audio|FadeOut (Variables|Default|GetAudio) 0.24 0.0 "Linear" :!class /Script/Engine.AudioComponent)
        (bind _returnvalue (Audio|SpawnSound2D (Variables|Default|GetAboveAmbient) 1.0 1.0 0.0 0))
        (Variables|Default|SetAudio _returnvalue)
        (Variables|Default|SetbIsPlayingBelowAmbient false)
        (Variables|Default|SetbIsPlayingAboveAmbient true))
      (elif (Variables|Default|GetbIsPlayingAboveAmbient)
        (Audio|Components|Audio|FadeOut (Variables|Default|GetAudio) 0.24 0.0 "Linear" :!class /Script/Engine.AudioComponent)
        (bind _returnvalue_2 (Audio|SpawnSound2D (Variables|Default|GetBelowAmbient) 1.0 1.0 0.0 0))
        (Variables|Default|SetAudio _returnvalue_2)
        (Variables|Default|SetbIsPlayingBelowAmbient true)
        (Variables|Default|SetbIsPlayingAboveAmbient false)))))

(event EventBeginPlay
  (bind _returnvalue (Audio|SpawnSound2D (Variables|Default|GetAboveAmbient) 1.0 1.0 0.0 0))
  (Variables|Default|SetAudio _returnvalue))

(event EventTick
  (params (DeltaSeconds :type Float%20%28single-precision%29)))

(fn ConstructionScript)