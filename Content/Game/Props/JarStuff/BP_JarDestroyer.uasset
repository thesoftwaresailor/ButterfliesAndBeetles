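; BP_JarDestroyer is a trigger actor that removes jars entering it and requests a replacement.
; On BeginPlay it finds and caches the BP_JarSpawner in the level.
; When a BP_Jar overlaps it, it calls the jar's PreparedDeath and then asks the cached spawner to spawn a new jar.
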(event EventBeginPlay
  (bind _returnvalue (Actor|GetActorOfClass "/Game/Game/Props/JarStuff/BP_JarSpawner.BP_JarSpawner_C"))
  (Variables|Default|SetJarSpawner _returnvalue))

(event Collision|EventActorBeginOverlap
  (params (OtherActor :type Actor%20Object%20Reference))
  (if (== (Utilities|GetClass OtherActor) "/Game/Game/Props/BP_Jar.BP_Jar_C")
    (bind _asbp_jar (Utilities|Casting|CastToBP_Jar OtherActor))
    (Default|PreparedDeath _asbp_jar)
    (Utilities|IsValid (Variables|Default|GetJarSpawner)
      (:Is%20Valid
        (Default|SpawnJar (Variables|Default|GetJarSpawner))))))

(event EventTick
  (params (DeltaSeconds :type Float%20%28single-precision%29)))

(fn ConstructionScript)