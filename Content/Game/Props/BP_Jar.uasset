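; BP_Jar is a VR jar prop that holds dead butterflies and keeps them inside when the player teleports.
; A cylinder overlap tracks the butterflies, and Tick attaches them to the jar while the Vive pawn, cached via a retry timer, teleports, detaching them otherwise.
; PreparedDeath expires the contents, calls the pawn's grip-or-drop using values stored by SetGripInfo, then destroys the jar on a timer once empty.
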(event OnComponentBeginOverlap(Cylinder)
  (params (OverlappedComponent :type Primitive%20Component%20Object%20Reference) (OtherActor :type Actor%20Object%20Reference) (OtherComp :type Primitive%20Component%20Object%20Reference) (OtherBodyIndex :type Integer) (bFromSweep :type Boolean) (SweepResult :type Hit%20Result%20Structure%20%28by%20ref%29))
  ;[1 1 1] Check if have butterflies inside
  (if (== (Utilities|GetClass OtherActor) "/Game/Game/Props/BP_DeadButterfly.BP_DeadButterfly_C")
    (Utilities|Array|AddUnique (Variables|Default|GetDeadbutterfly) OtherActor)))

(event OnComponentEndOverlap(Cylinder)
  (params (OverlappedComponent :type Primitive%20Component%20Object%20Reference) (OtherActor :type Actor%20Object%20Reference) (OtherComp :type Primitive%20Component%20Object%20Reference) (OtherBodyIndex :type Integer))
  ;[1 1 1] Check if have butterflies inside
  (if (== (Utilities|GetClass OtherActor) "/Game/Game/Props/BP_DeadButterfly.BP_DeadButterfly_C")
    (Utilities|Array|RemoveItem (Variables|Default|GetDeadbutterfly) OtherActor)))

(event Custom|GetPlayerPawn
  ;[1 1 1] Very 'professionally' get ref to pawn
  (bind _asvive_pawn_character (Utilities|Casting|CastToVive_PawnCharacter (Game|Player|GetPlayerPawn 0))
    (:then
      (Variables|Default|SetAs%20Vive%20Pawn%20Character _asvive_pawn_character))
    (:CastFailed
      (Utilities|Time|SetTimerbyEvent (delegate Custom|GetPlayerPawn) 0.5))))

(event Custom|PreparedDeath
  (bind _deadbutterfly (Variables|Default|GetDeadbutterfly))
  (for _array_element _deadbutterfly
    (Actor|SetLifeSpan _array_element 0.1)
    (Development|PrintString "DIE"))
  (Utilities|Array|Clear _deadbutterfly)
  (bind _asvive_pawn_character (Utilities|Casting|CastToVive_PawnCharacter (Game|Player|GetPlayerPawn 0))
    (:then
      (Default|GriporDropObjectClean _asvive_pawn_character (Variables|Default|GetCalling%20Motion%20Controller) (Variables|Default|GetOther%20Controller) (Variables|Default|GetCan%20Check%20Climb) (Variables|Default|GetGrab%20Sphere) "(GameplayTags=((TagName=\"DropType.OnPrimaryGripRelease\"),(TagName=\"DropType.Secondary.OnPrimaryGripRelease\")))"))
    (:CastFailed
      _))
  (Utilities|Time|SetTimerbyEvent (delegate Custom|death) 0.1 true))

(event Custom|death
  (if (== (Utilities|Array|Length (Variables|Default|GetDeadbutterfly)) 0)
    (Actor|DestroyActor)))

(event EventBeginPlay
  ;[1 1 1] Very 'professionally' get ref to pawn
  (bind _asvive_pawn_character (Utilities|Casting|CastToVive_PawnCharacter (Game|Player|GetPlayerPawn 0))
    (:then
      (Variables|Default|SetAs%20Vive%20Pawn%20Character _asvive_pawn_character))
    (:CastFailed
      (Utilities|Time|SetTimerbyEvent (delegate Custom|GetPlayerPawn) 0.5))))

(event EventTick
  (params (DeltaSeconds :type Float%20%28single-precision%29))
  (bind _as_vive_pawn_character (Variables|Default|GetAs%20Vive%20Pawn%20Character))
  ;[1 1 1] dirty and not efficent way to ensure objects stay inside jar if teleported when holding jar. Only works with dead butterflies. So, better hope they don't put other objects in here
  (if (> (Utilities|Array|Length (Variables|Default|GetDeadbutterfly)) 0)
    (Utilities|IsValid _as_vive_pawn_character
      (:Is%20Valid
        (if (Variables|/Game/VRExpansion/Vive/Vive_PawnCharacter.Vive_PawnCharacter_C|GetIsTeleporting _as_vive_pawn_character)
          (for _array_element (Variables|Default|GetDeadbutterfly)
            (Transformation|AttachActorToActor _array_element self "None" "KeepWorld" "KeepWorld" "KeepWorld" true))
          (else
            (for _array_element_2 (Variables|Default|GetDeadbutterfly)
              (Transformation|DetachFromActor _array_element_2 "KeepWorld" "KeepWorld" "KeepWorld"))))))))

(fn ConstructionScript)

(fn SetGripInfo
  (params (CallingMotionController :type Grip%20Motion%20Controller%20Component%20Object%20Reference) (OtherController :type Grip%20Motion%20Controller%20Component%20Object%20Reference) (CanCheckClimb :type Boolean) (GrabSphere :type Primitive%20Component%20Object%20Reference) (RelevantGameplayTags :type Gameplay%20Tag%20Container%20Structure))
  (Variables|Default|SetCalling%20Motion%20Controller CallingMotionController)
  (Variables|Default|SetOther%20Controller OtherController)
  (Variables|Default|SetCan%20Check%20Climb CanCheckClimb)
  (Variables|Default|SetGrab%20Sphere GrabSphere)
  (Variables|Default|SetRelevant%20Gameplay%20Tags RelevantGameplayTags))