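; Tutorial spawner actor that places a scaled-down BP_Jar at its own location on BeginPlay and advances the tutorial when a dead butterfly reaches it.
; It binds the jar cylinder's overlap, and the first BP_DeadButterfly contact plays a voice line, reveals the MoveInd indicator and sets HasDeadButterfly.
; Each SpawnJar call also spawns a dead butterfly at the spawner if that flag is already set.
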(event Custom|SpawnJar
  (bind _returnvalue (Game|SpawnActorfromClass "/Game/Game/Props/BP_Jar.BP_Jar_C" (Math|Transform|MakeTransform (Transformation|GetActorLocation) "0, 0, 0" "0.250000,0.250000,0.250000") "Undefined" 0 0))
  (Variables|Default|SetJar _returnvalue)
  (Collision|BindEventtoOnComponentBeginOverlap (Variables|/Game/Game/Props/BP_Jar.BP_Jar_C|GetCylinder (Variables|Default|GetJar)) (delegate Custom|HeadDownstairs))
  (CallFunction|SpawnButterfly))

(event Custom|SpawnButterfly
  (if (Variables|Default|GethasDeadButterfly)
    (Game|SpawnActorfromClass "/Game/Game/Props/BP_DeadButterfly.BP_DeadButterfly_C" (Math|Transform|MakeTransform (Transformation|GetActorLocation) "0, 0, 0" "1,1,1") "Undefined" 0 0)))

(event Custom|HeadDownstairs
  (params (OverlappedComponent :type Primitive%20Component%20Object%20Reference) (OtherActor :type Actor%20Object%20Reference) (OtherComp :type Primitive%20Component%20Object%20Reference) (OtherBodyIndex :type Integer) (bFromSweep :type Boolean) (SweepResult :type Hit%20Result%20Structure%20%28by%20ref%29))
  (if (and (== (Utilities|GetClass OtherActor) "/Game/Game/Props/BP_DeadButterfly.BP_DeadButterfly_C") (not (Variables|Default|GetbHasTriggeredGoDownstairs)))
    (Variables|Default|SethasDeadButterfly true)
    (Audio|SpawnSound2D (Variables|Default|GetVL-05) 1.0 1.0 0.0 0)
    (Default|BecomeVisible (Variables|Default|GetMoveInd))
    (Variables|Default|SetbHasTriggeredGoDownstairs true)))

(event EventBeginPlay
  (CallFunction|SpawnJar))

(event Collision|EventActorBeginOverlap
  (params (OtherActor :type Actor%20Object%20Reference)))

(event EventTick
  (params (DeltaSeconds :type Float%20%28single-precision%29)))

(fn ConstructionScript)