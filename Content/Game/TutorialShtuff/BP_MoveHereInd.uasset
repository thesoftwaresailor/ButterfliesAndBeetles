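; Tutorial "move here" indicator actor that bobs between two points and can be shown or hidden.
; From BeginPlay, a timeline lerps the MoveHere component between the Apex and Nadir positions, flipping direction and replaying on each finish to loop endlessly.
; BecomeVisible shows MoveHere and spawns a ding sound at the actor, and UnBecomeVisible hides it and stops that sound.
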(event Custom|BecomeVisible
  (Rendering|SetVisibility (Variables|Default|GetMoveHere) true false)
  (bind _returnvalue (Audio|SpawnSoundatLocation "/Game/Game/Sounds/EventDing_Cue.EventDing_Cue" (Transformation|GetActorLocation) "0, 0, 0" 1.0 1.0 0.0 0 0))
  (Variables|Default|SetDing _returnvalue))

(event Custom|UnBecomeVisible
  (Rendering|SetVisibility (Variables|Default|GetMoveHere) false false)
  (Audio|Components|Audio|Stop (Variables|Default|GetDing)))

(event Custom|Bob
  (if (Variables|Default|GetbMovingUp)
    (bind _bobtrack (Timeline|BobTimeline ReverseFromEnd)
      (:Update
        (Transformation|SetWorldLocation (Variables|Default|GetMoveHere) (Math|Vector|Lerp(Vector) (Transformation|GetWorldLocation (Variables|Default|GetApex)) (Transformation|GetWorldLocation (Variables|Default|GetNadir)) _bobtrack) false false))
      (:Finished
        (Variables|Default|SetbMovingUp (not (Variables|Default|GetbMovingUp)))
        (CallFunction|Bob)))
    (else
      (Timeline|BobTimeline PlayFromStart))))

(event EventBeginPlay
  (CallFunction|Bob))

(event Collision|EventActorBeginOverlap
  (params (OtherActor :type Actor%20Object%20Reference)))

(event EventTick
  (params (DeltaSeconds :type Float%20%28single-precision%29)))

(fn ConstructionScript)