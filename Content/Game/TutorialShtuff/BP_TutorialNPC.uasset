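; Tutorial NPC that takes on a random character mesh at BeginPlay and reacts to butterfly jars.
; Once it has arrived, an overlap on its ExtraHands component calls PreparedDeath on any BP_Jar holding at least one dead butterfly.
; Reach and BecomeVisible events set the reaching flag in AnimBP_NPC and unhide the actor.
; A note marks the jar count check as a swap point for an order game mode.
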(event OnComponentBeginOverlap(ExtraHands)
  (params (OverlappedComponent :type Primitive%20Component%20Object%20Reference) (OtherActor :type Actor%20Object%20Reference) (OtherComp :type Primitive%20Component%20Object%20Reference) (OtherBodyIndex :type Integer) (bFromSweep :type Boolean) (SweepResult :type Hit%20Result%20Structure%20%28by%20ref%29))
  (if (Variables|Default|GetbHasArrived)
    (bind _asbp_jar (Utilities|Casting|CastToBP_Jar OtherActor))
    (if (> (Utilities|Array|Length (Variables|/Game/Game/Props/BP_Jar.BP_Jar_C|GetDeadbutterfly _asbp_jar)) 0)
      (Default|PreparedDeath _asbp_jar))))

(event Custom|Reach
  (bind _asanim_bp_npc (Utilities|Casting|CastToAnimBP_NPC (Components|SkeletalMesh|GetAnimInstance (Variables|Character|GetMesh))))
  (Variables|/Game/PolygonFantasyKingdom/Anims/AnimBP_NPC.AnimBP_NPC_C|SetbReaching _asanim_bp_npc true))

(event Custom|BecomeVisible
  (Rendering|SetActorHiddenInGame false))

(event EventBeginPlay
  (CallFunction|ChooseRandomMesh))

(fn ConstructionScript)

(fn ChooseRandomMesh
  (bind _charactermeshes (Variables|Default|GetCharacterMeshes))
  (Class|SkinnedMeshComponent|SetSkeletalMesh (Variables|Character|GetMesh) (Utilities|Array|Get(acopy) _charactermeshes (Math|Random|RandomIntegerinRange 0 (Utilities|Array|LastIndex _charactermeshes))) true))