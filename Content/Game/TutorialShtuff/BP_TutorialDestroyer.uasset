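; BP_TutorialDestroyer is a tutorial overlap zone that disposes of jars and dead butterflies and asks for replacements.
; On BeginPlay it caches the BP_TutoriaJarSpawner found in the level.
; An overlapping BP_Jar gets PreparedDeath and triggers SpawnJar if the spawner is valid.
; An overlapping BP_DeadButterfly triggers SpawnButterfly, without that validity check, and is then destroyed.
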(event EventBeginPlay
  (bind _returnvalue (Actor|GetActorOfClass "/Game/Game/TutorialShtuff/BP_TutoriaJarSpawner.BP_TutoriaJarSpawner_C"))
  (Variables|Default|SetTutJarSpawner _returnvalue))

(event Collision|EventActorBeginOverlap
  (params (OtherActor :type Actor%20Object%20Reference))
  (bind _returnvalue (Utilities|GetClass OtherActor))
  (if (== _returnvalue "/Game/Game/Props/BP_Jar.BP_Jar_C")
    (bind _asbp_jar (Utilities|Casting|CastToBP_Jar OtherActor))
    (Default|PreparedDeath _asbp_jar)
    (Utilities|IsValid (Variables|Default|GetTutJarSpawner)
      (:Is%20Valid
        (Default|SpawnJar (Variables|Default|GetTutJarSpawner))))
    (elif (== _returnvalue "/Game/Game/Props/BP_DeadButterfly.BP_DeadButterfly_C")
      (Default|SpawnButterfly (Variables|Default|GetTutJarSpawner))
      (Actor|DestroyActor OtherActor))))

(event EventTick
  (params (DeltaSeconds :type Float%20%28single-precision%29)))

(fn ConstructionScript)